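; VR player character that keeps its capsule and body mesh under the headset as the player moves.
; Each tick it shifts the capsule to the camera's XY, counter-shifts the VR origin, and adjusts capsule half-height from camera height.
; The mesh and origin snap to capsule bottom.
; Enhanced Input moves along LMC's flattened forward vector; strafing and ceiling checks are disconnected, and the low-camera correction is zeroed.
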(event Input|EnhancedActionEvents|EnhancedInputActionIA_Move_Leilei
  (params (ActionValue :type Vector%202D%20Structure) (ElapsedSeconds :type Float%20%28double-precision%29) (TriggeredSeconds :type Float%20%28double-precision%29) (InputAction :type Input%20Action%20Object%20Reference :default "/Game/Input/Actions/IA_Move_Leilei.IA_Move_Leilei"))
  (Pawn|Input|AddMovementInput (Class|KismetMathLibrary|VectorNormal2D (Math|Vector|GetForwardVector (Variables|Default|GetLMC)) 0.0001) (.x ActionValue) false))

(event EventBeginPlay
  (Input|AddMappingContext (PlayerController|LocalPlayerSubsystems|GetEnhancedInputLocalPlayerSubsystem (Game|GetPlayerController 0)) "/Game/Input/VRInput_Leilei.VRInput_Leilei" 0 "(bIgnoreAllPressedKeysUntilRelease=True,bForceImmediately=False,bNotifyUserSettings=False)"))

(event Collision|EventActorBeginOverlap
  (params (OtherActor :type Actor%20Object%20Reference)))

(event EventTick
  (params (DeltaSeconds :type Float%20%28single-precision%29))
  (CallFunction|CalculateHMDOffset)
  (CallFunction|ApplyXYOffset)
  (CallFunction|ApplyZOffset))

(fn ConstructionScript)

(fn CalculateHMDOffset
  (Variables|Default|SetHMDOffset2 (- (Transformation|GetWorldLocation (Variables|Default|GetCamera2)) (Transformation|GetWorldLocation (Variables|Collision|GetCapsuleComponent)))))

(fn ApplyXYOffset
  (bind _hmdoffset2 (Variables|Default|GetHMDOffset2))
  (bind _vrorigin2 (Variables|Default|GetVROrigin2))
  (bind _hmdoffset2_2 (Variables|Default|GetHMDOffset2))
  (bind _capsulecomponent (Variables|Collision|GetCapsuleComponent))
  (bind _returnvalue (Transformation|GetWorldLocation _vrorigin2))
  (bind _returnvalue_2 (* _hmdoffset2_2 -1.0))
  (Transformation|AddWorldOffset (Variables|Collision|GetCapsuleComponent) (Math|Vector|MakeVector (.x _hmdoffset2) (.y _hmdoffset2) 0.0) false false)
  (Transformation|AddWorldOffset _vrorigin2 (Math|Vector|MakeVector (.x _returnvalue_2) (.y _returnvalue_2) 0.0) false false)
  (Transformation|SetWorldLocation _vrorigin2 (Math|Vector|MakeVector (.x _returnvalue) (.y _returnvalue) (- (.z (Transformation|GetWorldLocation _capsulecomponent)) (Components|Capsule|GetScaledCapsuleHalfHeight _capsulecomponent))) false false))

(fn ApplyZOffset
  (CallFunction|CheckBottom)
  (CallFunction|CaulculateHalfHeight)
  (CallFunction|UpdateMeshLocationandRotation))

(fn CheckBottom
  (bind _output_get (LocalVariables|SetCameraHeightOffset2 (- (.z (Transformation|GetWorldLocation (Variables|Default|GetCamera2))) (.z (Transformation|GetWorldLocation (Variables|Collision|GetCapsuleComponent))))))
  (if (< _output_get 0.0)
    (Transformation|AddWorldOffset (Variables|Default|GetVROrigin2) (Math|Vector|MakeVector 0.0 0.0 (* _output_get 0.0)) false false)))

(fn CheckTop
  (bind _capsulecomponent (Variables|Collision|GetCapsuleComponent))
  (bind _capsulecomponent_2 (Variables|Collision|GetCapsuleComponent))
  (bind _returnvalue (Transformation|GetWorldLocation _capsulecomponent_2))
  (bind _returnvalue_2 (Transformation|GetWorldLocation _capsulecomponent))
  (bind (_x _y _z) (Math|Vector|BreakVector _returnvalue_2))
  (bind (_x_2 _y_2) (Math|Vector|BreakVector _returnvalue))
  (Utilities|FlowControl|Sequence
    (:then_0
      (bind (_outhit _returnvalue_3) (Collision|LineTraceByChannel _returnvalue (Math|Vector|MakeVector _x_2 _y_2 (+ (Components|Capsule|GetScaledCapsuleRadius _capsulecomponent_2) (.z (Transformation|GetWorldLocation (Variables|Default|GetCamera2))))) "TraceTypeQuery1" false 0 "None"))
      (if _returnvalue_3
        (Components|Capsule|SetCapsuleHalfHeight (Variables|Collision|GetCapsuleComponent) (- (.Distance (Collision|BreakHitResult _outhit)) 0.1) true)
        (Transformation|AddWorldOffset (Variables|Default|GetVROrigin2) (Math|Vector|MakeVector 0.0 0.0 (- (.Z (Math|Vector|BreakVector (.Location (Collision|BreakHitResult _outhit)))) (+ (.z (Transformation|GetWorldLocation (Variables|Default|GetCamera2))) (Class|CapsuleComponent|GetUnscaledCapsuleRadius (Variables|Collision|GetCapsuleComponent))))) false false)))
    (:then_1
      (bind (_outhit_2 _returnvalue_4) (Collision|LineTraceByChannel _returnvalue_2 (Math|Vector|MakeVector _x _y (- _z (Components|Capsule|GetScaledCapsuleHalfHeight _capsulecomponent))) "TraceTypeQuery1" false 0 "None"))
      (if _returnvalue_4
        (Components|Capsule|SetCapsuleHalfHeight (Variables|Collision|GetCapsuleComponent) (- (.Distance (Collision|BreakHitResult _outhit_2)) 0.1) true)))))

(fn UpdateMeshLocationandRotation
  (bind _capsulecomponent (Variables|Collision|GetCapsuleComponent))
  (bind _returnvalue (Transformation|GetWorldLocation _capsulecomponent))
  (Transformation|SetWorldLocation (Variables|Character|GetMesh) (Math|Vector|MakeVector (.x _returnvalue) (.y _returnvalue) (- (.z _returnvalue) (Components|Capsule|GetScaledCapsuleHalfHeight _capsulecomponent))) false false))

(fn CaulculateHalfHeight
  (bind _capsulecomponent (Variables|Collision|GetCapsuleComponent))
  (bind _returnvalue (Components|Capsule|GetScaledCapsuleHalfHeight _capsulecomponent))
  (Components|Capsule|SetCapsuleHalfHeight (Variables|Collision|GetCapsuleComponent) (/ (+ (- (.z (Transformation|GetWorldLocation (Variables|Default|GetCamera2))) (- (.z (Transformation|GetWorldLocation _capsulecomponent)) _returnvalue)) _returnvalue) 2.0) true))

(fn SetMesh)